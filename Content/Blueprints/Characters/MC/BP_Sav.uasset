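; Player character that runs a three-level timed game, teleporting between level and default locations and driving the overlay timer.
; A Delay-gated Tick countdown calls each level's completion, which checks artifact and anti-mind-control counts.
; Low counts darken tagged lights, enable unbound post-processing or spawn doors in later levels, and select companion or enemy dialogue widgets.
; Level three builds a dialogue queue for the ending; keys 1 and 2 increment both counters.
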(event EventBeginPlay)

(event Collision|EventActorBeginOverlap
  (params (OtherActor :type Actor%20Object%20Reference)))

(event EventTick
  (params (DeltaSeconds :type Float%20%28single-precision%29))
  (if (Variables|Default|GetTimerIsRunning)
    (Utilities|FlowControl|Delay 1.0)
    (if (== (Variables|Default|GetSeconds) 0)
      (if (== (Variables|Default|GetMinutes) 0)
        (Variables|Default|SetTimerIsRunning false)
        (switch int (Variables|Default|GetCurrentLevel)
          (:1
            (Development|PrintString "About to call completelevelone")
            (CallFunction|CompleteLevelOne))
          (:2
            (Development|PrintString "About to call completeleveltwo")
            (CallFunction|CompleteLevelTwo))
          (:3
            (Development|PrintString "About to call completelevelthree")
            (CallFunction|CompleteLevelThree)))
        (else
          (Variables|Default|SetSeconds 60)
          (Variables|Default|SetMinutes (- (Variables|Default|GetMinutes) 1))
          (Default|UpdateTimer (Variables|Default|GetOverlay) (Variables|Default|GetMinutes) (Variables|Default|GetSeconds))))
      (else
        (Variables|Default|SetSeconds (- (Variables|Default|GetSeconds) 1))
        (Default|UpdateTimer (Variables|Default|GetOverlay) (Variables|Default|GetMinutes) (Variables|Default|GetSeconds))))))

(event Input|KeyboardEvents|1
  (params (Key :type Key%20Structure :default "None"))
  (:Pressed
    (Class|Savior|IncreaseArtifacts)))

(event Input|KeyboardEvents|2
  (params (Key :type Key%20Structure :default "None"))
  (:Pressed
    (Class|Savior|IncreaseAMC)))

(fn ConstructionScript)

(fn StartLevelOne
  (bind _overlay (Variables|Default|GetOverlay))
  (Transformation|SetActorLocation (Variables|Default|GetLocationLevel1) false true)
  (Pawn|SetControlRotation (Game|GetPlayerController 0) (Variables|Default|GetRotationLevel1))
  (Variables|Default|SetCurrentLevel 1)
  (bind _output_get (Variables|Default|SetSeconds 19))
  (Default|UpdateTimer _overlay 0 _output_get)
  (Default|SetTimerVisible _overlay "Visible")
  (Variables|Default|SetTimerIsRunning true))

(fn CompleteLevelOne
  (bind _returnvalue (Game|GetPlayerController 0))
  (bind _returnvalue_2 (Class|Savior|GetAntiMindControlCount))
  (Input|SetInputModeUIOnly _returnvalue 0 "LockAlways")
  (Transformation|SetActorLocation (Variables|Default|GetDefaultLocation) false true)
  (Pawn|SetControlRotation _returnvalue (Variables|Default|GetDefaultRotation))
  (Default|SetTimerVisible (Variables|Default|GetOverlay) "Hidden")
  (if (< (Class|Savior|GetArtifactCount) 7)
    (CallFunction|SpawnLevelTwoPunishment))
  (Variables|Default|SetBaseMCCount _returnvalue_2)
  (if (== _returnvalue_2 0)
    (CallFunction|CreateEnemyWidget "/Game/Blueprints/HUD/PostLevel1/WBP_EnemyD_PostLevel1.WBP_EnemyD_PostLevel1_C")
    (CallFunction|SpawnLevelTwoNoReward)
    (else
      (Default|UpdateCompanionHealth (Variables|Default|GetOverlay) (* (Math|Conversions|ToFloat(Integer) (Class|Savior|GetAntiMindControlCount)) 0.2))
      (CallFunction|CreateCompanionWidget "/Game/Blueprints/HUD/PostLevel1/WBP_CompD_PostLevel1.WBP_CompD_PostLevel1_C"))))

(fn SetOverlay
  (params (InOverlay :type WBP%20Overlay%20Object%20Reference))
  (Variables|Default|SetOverlay InOverlay))

(fn StartLevelTwo
  (bind _overlay (Variables|Default|GetOverlay))
  (Class|Savior|ClearItemCounters)
  (Transformation|SetActorLocation (Variables|Default|GetLocationLevel2) false true)
  (Pawn|SetControlRotation (Game|GetPlayerController 0) (Variables|Default|GetRotationLevel2))
  (Variables|Default|SetCurrentLevel 2)
  (bind _output_get (Variables|Default|SetSeconds 40))
  (Default|UpdateTimer _overlay 0 _output_get)
  (Default|SetTimerVisible _overlay "Visible")
  (Variables|Default|SetTimerIsRunning true))

(fn CompleteLevelTwo
  (bind _returnvalue (Class|Savior|GetAntiMindControlCount))
  (Transformation|SetActorLocation (Variables|Default|GetDefaultLocation) false true)
  (Pawn|SetControlRotation (Game|GetPlayerController 0) (Variables|Default|GetDefaultRotation))
  (Default|SetTimerVisible (Variables|Default|GetOverlay) "Hidden")
  (if (> (Variables|Default|GetBaseMCCount) 0)
    (bind _returnvalue_2 (UserInterface|CreateWidget "/Game/Blueprints/HUD/PostLevel2/WBP_CompD_PostLevel2_1.WBP_CompD_PostLevel2_1_C" 0 _returnvalue))
    (CallFunction|CreateCompanionWidget 0 _returnvalue_2)
    (bind _output_get (Variables|Default|SetBaseMCCount (+ (Class|Savior|GetAntiMindControlCount) (Variables|Default|GetBaseMCCount)) :!label _label))
    (Default|UpdateCompanionHealth (Variables|Default|GetOverlay) (* (Math|Conversions|ToFloat(Integer) (Class|Savior|GetAntiMindControlCount)) 0.2))
    (elif (== _returnvalue 0)
      (Development|PrintString "About to create Enemy Widget for Post Level 2")
      (CallFunction|CreateEnemyWidget "/Game/Blueprints/HUD/PostLevel2/WBP_EnemyD_PostLevel2.WBP_EnemyD_PostLevel2_C")
      (else
        (CallFunction|CreateCompanionWidget "/Game/Blueprints/HUD/PostLevel2/WBP_CompD_PostLevel2_2.WBP_CompD_PostLevel2_2_C")
        (goto _label))))
  (if (> _output_get 2)
    _
    (else
      (CallFunction|SpawnLevelThreeNoReward)))
  (if (< (Class|Savior|GetArtifactCount) 9)
    (CallFunction|SpawnLevelThreePunishment)))

(fn StartLevelThree
  (bind _overlay (Variables|Default|GetOverlay))
  (Development|PrintString "In StartLevelThree")
  (Class|Savior|ClearItemCounters)
  (Transformation|SetActorLocation (Variables|Default|GetLocationLevel3) false true)
  (Pawn|SetControlRotation (Game|GetPlayerController 0) (Variables|Default|GetRotationLevel3))
  (Variables|Default|SetCurrentLevel 3)
  (bind _output_get (Variables|Default|SetSeconds 40))
  (Default|UpdateTimer _overlay 0 _output_get)
  (Default|SetTimerVisible _overlay "Visible")
  (Variables|Default|SetTimerIsRunning true))

(fn CompleteLevelThree
  (bind _returnvalue (Class|Savior|GetAntiMindControlCount))
  (bind _newdialoguequeue (Variables|Default|GetNewDialogueQueue))
  (bind _basemccount (Variables|Default|GetBaseMCCount))
  (bind _returnvalue_2 (Actor|GetActorOfClass "/Script/Engine.PostProcessVolume"))
  (Variables|/Script/Engine.PostProcessVolume|SetbUnbound _returnvalue_2 false)
  (Transformation|SetActorLocation (Variables|Default|GetDefaultLocation) false true)
  (Pawn|SetControlRotation (Game|GetPlayerController 0) (Variables|Default|GetDefaultRotation))
  (Default|SetTimerVisible (Variables|Default|GetOverlay) "Hidden")
  ;[1 1 1] Companion: Which Dialogues should the user see, based on theri performance throughout the game? Which ending will they receive?
  (if (== _basemccount 0)
    (if (== (Class|Savior|GetAntiMindControlCount) 0)
      _
      (else
        ;;[1 1 1] You give LS the first dose
        (bind _returnvalue_3 (UserInterface|CreateWidget "/Game/Blueprints/HUD/PostLevel3/WBP_Comp_C1_L3.WBP_Comp_C1_L3_C"))
        (Utilities|Array|Add (Variables|Default|GetNewDialogueQueue) _returnvalue_3)))
    ;[1 1 1] Only one Enemy ending: Push it
    (bind _returnvalue_4 (UserInterface|CreateWidget "/Game/Blueprints/HUD/PostLevel3/WBP_Enemy_E1_L3.WBP_Enemy_E1_L3_C" :!label _label))
    (Utilities|Array|Add (Variables|Default|GetNewDialogueQueue) _returnvalue_4)
    (if (>= (Class|Savior|GetTotalArtifactCount) 29)
      ;[1 1 1] Add "You Won... kind of" dialogue
      (bind _returnvalue_5 (UserInterface|CreateWidget "/Game/Blueprints/HUD/PostLevel3/Endings/WBP_L3_YouWon_Sorta.WBP_L3_YouWon_Sorta_C"))
      (Utilities|Array|Add (Variables|Default|GetNewDialogueQueue) _returnvalue_5)
      (else
        ;[1 1 1] Add "Game Over" dialogue
        (bind _returnvalue_6 (UserInterface|CreateWidget "/Game/Blueprints/HUD/PostLevel3/Endings/WBP_L3_GameOver.WBP_L3_GameOver_C"))
        (Utilities|Array|Add (Variables|Default|GetNewDialogueQueue) _returnvalue_6)))
    (else
      ;;[1 1 1] Display 'did you see the things I did for you' but only if LS's MC is sufficiently cleared
      (if (> _basemccount 2)
        (Development|PrintString "Prev > 2; Adding C2L3")
        (bind _returnvalue_7 (UserInterface|CreateWidget "/Game/Blueprints/HUD/PostLevel3/WBP_Comp_C2_L3.WBP_Comp_C2_L3_C"))
        (Utilities|Array|Add (Variables|Default|GetNewDialogueQueue) _returnvalue_7))
      (if (== _returnvalue 0)
        (goto _label)
        (elif (>= (+ _returnvalue (Variables|Default|GetBaseMCCount)) 5)
          ;;[1 1 1] Display "LightSong breaks free and the two of you devastate the room and fly away
          (bind _returnvalue_8 (UserInterface|CreateWidget "/Game/Blueprints/HUD/PostLevel3/WBP_Comp_C4_L3.WBP_Comp_C4_L3_C"))
          (Utilities|Array|Add _newdialoguequeue _returnvalue_8)
          (bind _returnvalue_9 (UserInterface|CreateWidget "/Game/Blueprints/HUD/PostLevel3/Endings/WBP_L3_YouWon.WBP_L3_YouWon_C"))
          (Utilities|Array|Add _newdialoguequeue _returnvalue_9)
          (else
            ;;[1 1 1] Display followup "You give LS her new doses" Dialogue
            (bind _returnvalue_10 (UserInterface|CreateWidget "/Game/Blueprints/HUD/PostLevel3/WBP_Comp_C3_L3.WBP_Comp_C3_L3_C"))
            (Utilities|Array|Add (Variables|Default|GetNewDialogueQueue) _returnvalue_10)
            (goto _label))))))
  ;[1 1 1] Update LS's Health Overlay
  (Default|UpdateCompanionHealth (Variables|Default|GetOverlay) (* (Math|Conversions|ToFloat(Integer) (Class|Savior|GetAntiMindControlCount)) 0.2))
  (CallFunction|ShowLevelThreeDialogues))

(fn CreateCompanionWidget
  (params (InWidgetClass :type User%20Widget%20Class%20Reference) (InWidget :type User%20Widget%20Object%20Reference))
  (bind _returnvalue (Game|GetPlayerController 0))
  (bind _returnvalue_2 (Viewport|GetViewportSize))
  (if (== InWidget 0)
    (bind _returnvalue_3 (UserInterface|CreateWidget InWidgetClass))
    (LocalVariables|SetCurrentWidget _returnvalue_3)
    (else
      (LocalVariables|SetCurrentWidget InWidget)))
  (Class|UserWidget|SetPositioninViewport (LocalVariables|GetCurrentWidget) (Math|Vector2D|MakeVector2D (/ (.x _returnvalue_2) 1.8) (/ (.y _returnvalue_2) 2.5)) true)
  (Class|UserWidget|SetDesiredSizeinViewport (LocalVariables|GetCurrentWidget) "(X=500.000000,Y=400.000000)")
  (UserInterface|Viewport|AddtoViewport (LocalVariables|GetCurrentWidget) 0)
  (Widget|SetFocus (LocalVariables|GetCurrentWidget))
  (Input|SetInputModeUIOnly _returnvalue (LocalVariables|GetCurrentWidget) "DoNotLock")
  (Variables|/Script/Engine.PlayerController|SetbShowMouseCursor _returnvalue true))

(fn CreateEnemyWidget
  (params (InWidget :type User%20Widget%20Class%20Reference))
  (bind _returnvalue (Game|GetPlayerController 0))
  (bind _returnvalue_2 (UserInterface|CreateWidget InWidget))
  (Class|UserWidget|SetPositioninViewport _returnvalue_2 (Math|Vector2D|MakeVector2D (LocalVariables|GetX) (/ (.y (Viewport|GetViewportSize)) 2.0)) true)
  (Variables|Default|SetWidgetToCreate _returnvalue_2)
  (Class|UserWidget|SetDesiredSizeinViewport _returnvalue_2 "(X=500.000000,Y=400.000000)")
  (UserInterface|Viewport|AddtoViewport _returnvalue_2 0)
  (Widget|SetFocus _returnvalue_2)
  (Input|SetInputModeUIOnly _returnvalue _returnvalue_2 "DoNotLock")
  (Variables|/Script/Engine.PlayerController|SetbShowMouseCursor _returnvalue true))

(fn ShowLevelThreeDialogues
  (bind _returnvalue (Game|GetPlayerController 0))
  (bind _newdialoguequeue (Variables|Default|GetNewDialogueQueue))
  (Development|PrintString "In ShowLevelThreeDialogues")
  (Input|SetInputModeUIOnly _returnvalue 0 "DoNotLock")
  (Variables|/Script/Engine.PlayerController|SetbShowMouseCursor _returnvalue true)
  (if (Utilities|Array|IsNotEmpty (Variables|Default|GetNewDialogueQueue))
    (Default|DisplayWidget (Utilities|Array|Get(acopy) _newdialoguequeue))
    (Utilities|Array|RemoveIndex _newdialoguequeue)
    (else
      (Development|PrintString "Array is empty"))))

(fn SpawnLevelTwoPunishment
  (bind _outactors (Actor|GetAllActorsOfClasswithTag "/Script/Engine.PointLight" "Punishment2"))
  (for _array_element _outactors
    (Rendering|Components|Light|SetIntensity (Variables|/Script/Engine.Light|GetLightComponent _array_element) 0.0)))

(fn SpawnLevelTwoNoReward
  (Game|SpawnActorfromClass "/Game/Blueprints/Items/BP_Door.BP_Door_C" (LocalVariables|GetDoorTransform1) "AlwaysSpawn" 0 0)
  (Game|SpawnActorfromClass "/Game/Blueprints/Items/BP_Door.BP_Door_C" (LocalVariables|GetDoorTransform2) "AlwaysSpawn" 0 0)
  (Game|SpawnActorfromClass "/Game/Blueprints/Items/BP_Door.BP_Door_C" (LocalVariables|GetDoorTransform3) "AlwaysSpawn" 0 0)
  (Game|SpawnActorfromClass "/Game/Blueprints/Items/BP_Door.BP_Door_C" (LocalVariables|GetDoorTransform4) "AlwaysSpawn" 0 0))

(fn SpawnLevelThreeNoReward
  (Game|SpawnActorfromClass "/Game/Blueprints/Items/BP_Door.BP_Door_C" (LocalVariables|GetDoorTransform5) "AlwaysSpawn" 0 0)
  (Game|SpawnActorfromClass "/Game/Blueprints/Items/BP_Door.BP_Door_C" (LocalVariables|GetDoorTransform6) "AlwaysSpawn" 0 0))

(fn SpawnLevelThreePunishment
  (bind _outactors (Actor|GetAllActorsOfClasswithTag "/Script/Engine.PointLight" "Punishment"))
  (for _array_element _outactors
    (Rendering|Components|Light|SetIntensity (Variables|/Script/Engine.Light|GetLightComponent _array_element) 0.0)
    (bind _returnvalue (Actor|GetActorOfClass "/Script/Engine.PostProcessVolume"))
    (Variables|/Script/Engine.PostProcessVolume|SetbUnbound _returnvalue true)))